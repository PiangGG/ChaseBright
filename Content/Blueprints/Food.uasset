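; Food is a randomized pickup actor that a Player consumes on overlap with its static mesh.
; The construction script picks a random mesh, randomizes material color and size parameters, and passes a random color and the mesh to the Eated1 Niagara component.
; On overlap, Eated calls the Player's Eat with itself, plays a random sound at its location, enables Niagara rendering, then immediately destroys the actor.
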(event `self.StaticMesh.OnComponentBeginOverlap`
  (params (OverlappedComponent :type "PrimitiveComponent Object Reference") (OtherActor :type "Actor Object Reference") (OtherComp :type "PrimitiveComponent Object Reference") (OtherBodyIndex :type Integer) (bFromSweep :type Boolean) (SweepResult :type "HitResult Structure (by ref)"))
  (`self.Eated` OtherActor))

(event `self.Eated1.OnComponentEndOverlap`
  (params (OverlappedComponent :type "PrimitiveComponent Object Reference") (OtherActor :type "Actor Object Reference") (OtherComp :type "PrimitiveComponent Object Reference") (OtherBodyIndex :type Integer)))

(fn `Eated`
  (params (Pawn :type "Actor Object Reference"))
  (bind _sound (`self.Sound`))
  (bind _asplayer (cast `/Game/GamePlay/Pawn/Player` Pawn))
  (`/Game/GamePlay/Pawn/Player.Eat` _asplayer self)
  (`GameplayStatics.SpawnSoundAtLocation` (`|GetArrayItem` _sound (`KismetMathLibrary.RandomInteger` (`KismetArrayLibrary.Array_Length` _sound))) (`self.K2_GetActorLocation`) (struct) 1.0 1.0 0.0 null null)
  (`NiagaraComponent.SetRenderingEnabled` (`self.Eated1`) true)
  (`self.K2_DestroyActor`))

(fn `UserConstructionScript`
  (bind _returnvalue (`KismetMathLibrary.RandomUnitVector`))
  (bind _mesharray (`self.MeshArray`))
  (bind _staticmesh (`self.StaticMesh`))
  (bind _eated1 (`self.Eated1`))
  (`StaticMeshComponent.SetStaticMesh` _staticmesh (`|GetArrayItem` _mesharray (`KismetMathLibrary.RandomInteger` (`KismetArrayLibrary.Array_Length` _mesharray))))
  (set `self.Color` _returnvalue)
  (`MeshComponent.SetVectorParameterValueOnMaterials` _staticmesh "Color4" _returnvalue)
  (`MeshComponent.SetScalarParameterValueOnMaterials` _staticmesh "Size" (* (`KismetMathLibrary.RandomFloat`) 100.0))
  (`NiagaraComponent.SetVariableVec3` _eated1 "Color_" _returnvalue)
  (`NiagaraFunctionLibrary.OverrideSystemUserVariableStaticMeshComponent` _eated1 "Mesh_" (`self.StaticMesh`)))